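; XR game mode that runs a timed, round-based score game with a persistent high score.
; BeginPlay loads the saved record from the "Record" slot, then starts a looping one-second countdown that quits the game when time runs out.
; AddScore raises the score, saves any new record immediately, and on reaching a growing threshold advances the round and refills the timer.
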(event `self.ReceiveBeginPlay`
  (`GameplayStatics.DoesSaveGameExist` "Record")
  (if true
    (bind _returnvalue (`GameplayStatics.LoadGameFromSlot` "Record"))
    (bind _asbp_max_score_sav (cast `/Game/BluePrint/BP_MaxScoreSav` _returnvalue))
    (set `self.Max Score Local` (`/Game/BluePrint/BP_MaxScoreSav.Max Score` _asbp_max_score_sav)))
  (set `self.Current Time` (`self.Round Time`))
  (`KismetSystemLibrary.K2_SetTimerDelegate` (delegate `Decrease Time`) 1.0 true))

(event `Decrease Time`
  (set `self.Current Time` (- (`self.Current Time`) 1.0))
  (if (<= (`self.Current Time`) 0.0)
    (`self.Game Over1`)))

(event `Game Over1`
  (`KismetSystemLibrary.PrintString` "GAME OVER")
  (`KismetSystemLibrary.QuitGame` null "Quit"))

(fn `Add Score`
  (params (`Points To Add` :type Integer))
  (set `self.Current Score` (+ (`self.Current Score`) `Points To Add`))
  (if (> (`self.Current Score`) (`self.Max Score Local`))
    (set `self.Max Score Local` (`self.Current Score`))
    (bind _returnvalue (`GameplayStatics.CreateSaveGameObject` "/Game/BluePrint/BP_MaxScoreSav.BP_MaxScoreSav_C"))
    (set `/Game/BluePrint/BP_MaxScoreSav.Max Score` (`self.Max Score Local`) _returnvalue)
    (`GameplayStatics.SaveGameToSlot` _returnvalue "Record"))
  (if (>= (`self.Current Score`) (`self.Score Thershold`))
    (set `self.Round` (+ (`self.Round`) 1))
    (set `self.Current Time` (`self.Round Time`))
    (set `self.Score Thershold` (+ (`self.Score Thershold`) 10))))

(fn `Game Over`)

(fn `UserConstructionScript`)