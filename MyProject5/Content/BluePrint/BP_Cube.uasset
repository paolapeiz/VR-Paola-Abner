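; BP_Cube is an actor with a cube component that destroys itself when a BP_Projectile overlaps it.
; On Tick, while CanJump is true, it applies a randomized velocity-change impulse to the cube, always upward and varied horizontally.
; It then clears CanJump, and nothing in this Blueprint sets it again.
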(event `self.ReceiveBeginPlay`)

(event `self.ReceiveActorBeginOverlap`
  (params (OtherActor :type "Actor Object Reference"))
  (cast `/Game/XRFramework/Blueprints/BP_Projectile` OtherActor)
  (`self.K2_DestroyActor`))

(event `self.ReceiveTick`
  (params (DeltaSeconds :type "Float (single-precision)"))
  (bind _vector (`self.Vector`))
  (if (`self.CanJump`)
    (`KismetMathLibrary.Vector_Set` _vector (`KismetMathLibrary.RandomFloatInRange` 0.0 750.0) (`KismetMathLibrary.RandomFloatInRange` -750.0 750.0) (`KismetMathLibrary.RandomFloatInRange` 100.0 750.0))
    (`PrimitiveComponent.AddImpulse` (`self.Cube`) _vector "None" true)
    (set `self.CanJump` false)))

(fn `UserConstructionScript`)