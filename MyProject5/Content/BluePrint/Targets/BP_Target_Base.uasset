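; BP_Target_Base is a scoring target for an XR game that can be hit by an axe weapon or a projectile.
; On BeginPlay it starts a timer that destroys the target once its configured lifetime runs out.
; On overlap with BP_Weapon_Axe or BP_Projectil, both checks share one path that adds the target's points through BP_XRGameMode, then destroys it.
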(event `Desapear`
  (`self.K2_DestroyActor`))

(event `self.ReceiveBeginPlay`
  (`KismetSystemLibrary.K2_SetTimerDelegate` (delegate `Desapear`) (`self.Target time life`)))

(event `self.ReceiveActorBeginOverlap`
  (params (OtherActor :type "Actor Object Reference"))
  (`|ExecutionSequence`
    (:`then_0`
      (cast `/Game/BluePrint/Weapon/BP_Weapon_Axe` OtherActor))
    (:`then_1`
      (cast `/Game/BluePrint/Weapon/BP_Projectil` OtherActor)))
  (bind _asbp_xrgame_mode (cast `/Game/XRFramework/Blueprints/BP_XRGameMode` (`GameplayStatics.GetGameMode`)))
  (`/Game/XRFramework/Blueprints/BP_XRGameMode.Add Score` _asbp_xrgame_mode (`self.Points`))
  (`self.K2_DestroyActor`))

(fn `UserConstructionScript`)