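; Target spawner actor that periodically spawns either a Civilian or an Enemy at a random point inside its SpawnArea box.
; StartSpawn_Event runs Generate on a looping timer at SpawnInterval, and each tick calls SpawnTarget, which picks the class by coin flip.
; PauseSpawn_Event re-sets the same timer event with no time given, which clears the timer if that time is zero.
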(event `self.ReceiveBeginPlay`)

(event `Generate`
  (`self.Spawn Target`))

(event `StartSpawn_Event`
  (`KismetSystemLibrary.K2_SetTimerDelegate` (delegate `Generate`) (`self.Spawn Interval`) true))

(event `PauseSpawn_Event`
  (`KismetSystemLibrary.K2_SetTimerDelegate` (delegate `Generate`) 0.0 true))

(fn `Spawn Target`
  (bind _spawn_area (`self.Spawn Area`))
  (bind _spawn_area_2 (`self.Spawn Area`))
  (if (`KismetMathLibrary.RandomBool`)
    (`|SpawnActorFromClass` (`self.Civilian`) (`KismetMathLibrary.MakeTransform` (`KismetMathLibrary.RandomPointInBoundingBox` (`SceneComponent.K2_GetComponentLocation` _spawn_area_2) (`BoxComponent.GetUnscaledBoxExtent` _spawn_area_2))) "Undefined" "MultiplyWithRoot" null null)
    (else
      (`|SpawnActorFromClass` (`self.Enemy`) (`KismetMathLibrary.MakeTransform` (`KismetMathLibrary.RandomPointInBoundingBox` (`SceneComponent.K2_GetComponentLocation` _spawn_area) (`BoxComponent.GetUnscaledBoxExtent` _spawn_area))) "Undefined" "MultiplyWithRoot" null null))))

(fn `UserConstructionScript`)