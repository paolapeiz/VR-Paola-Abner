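; BP_Weapon_Axe is an axe weapon Blueprint that is held by a motion-controller hand and destroys itself after a shot.
; AfterShoot, its only active custom logic, finds the owner of the grab component's motion controller and sends it a message to unhide the holding hand, right or left, before destroying the actor.
; The event graph holds only disabled stubs, and the construction script just calls the parent.
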(fn `AfterShoot`
  (bind _grabcomponentsnap (`self.GrabComponentSnap`))
  (message `/Game/XRFramework/Blueprints/BPI_PawnAnim.HideUnhideHand` (`ActorComponent.GetOwner` (`/Game/XRFramework/Blueprints/BP_GrabComponent.MotionControllerRef` _grabcomponentsnap)) false (`|EnumEquality` (`/Game/XRFramework/Blueprints/BP_GrabComponent.GetHeldByHand` _grabcomponentsnap) "Right"))
  (`self.K2_DestroyActor`))

(fn `UserConstructionScript`
  (`parent.UserConstructionScript`))