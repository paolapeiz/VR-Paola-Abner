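; BPC_Ammunition is a weapon Blueprint that tracks the rounds in the current magazine.
; Shoot checks whether rounds remain, decrements the count if so, and returns whether the shot is allowed.
; Reload refills the magazine to its capacity, with no reserve ammo pool.
; The event graph holds no active logic, so all behavior runs through these two functions.
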(fn `Reload`
  (set `self.CurrentMagazine` (`self.MagazinecCapacity`))
  (return))

(fn `Shoot`
  (returns (CanShoot :type Boolean))
  (bind _output_get (set `self.CanShoot` (> (`self.CurrentMagazine`) 0)))
  (if _output_get
    (`/Engine/EditorBlueprintResources/StandardMacros.DecrementInt` (`self.CurrentMagazine`)
      (:`  `
        _)))
  (return (`self.CanShoot`)))