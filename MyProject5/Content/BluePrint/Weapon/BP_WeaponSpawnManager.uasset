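; BP_WeaponSpawnManager is a manager that places weapons at the level's weapon spawn points and replaces them when grabbed.
; On BeginPlay it gathers every BP_WeaponSpawnPoint and calls the spawn event for each.
; The spawn event creates an actor from the point's WeaponClass at that point's transform.
; A weapon-grabbed event calls the same spawn event for the passed point after a short delay.
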(event `self.ReceiveBeginPlay`
  (bind _outactors (`GameplayStatics.GetAllActorsOfClass` "/Game/BluePrint/Weapon/BP_WeaponSpawnPoint.BP_WeaponSpawnPoint_C"))
  (bind _output_get (set `self.SpawnPoints` _outactors))
  (for _array_element _output_get
    (bind _asbp_weapon_spawn_point (cast `/Game/BluePrint/Weapon/BP_WeaponSpawnPoint` _array_element))
    (`self.SpawnWeapon_Event` _asbp_weapon_spawn_point)))

(event `SpawnWeapon_Event`
  (params (ObjectivePoint :type "/Game/BluePrint/Weapon/BP_WeaponSpawnPoint Object Reference"))
  (`|SpawnActorFromClass` (`GameplayStatics.GetObjectClass` (`/Game/BluePrint/Weapon/BP_WeaponSpawnPoint.WeaponClass` ObjectivePoint)) (`self.GetTransform` ObjectivePoint) "Undefined" "MultiplyWithRoot" null null))

(event `WeaponGrabbed_Event`
  (params (NewParam :type "/Game/BluePrint/Weapon/BP_WeaponSpawnPoint Object Reference"))
  (`KismetSystemLibrary.Delay` 0.1)
  (`self.SpawnWeapon_Event` NewParam))

(fn `UserConstructionScript`)